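; BP_Grotto is the player character, with side-scrolling style movement along the world X axis and jumping.
; BeginPlay registers the IMC_Player Enhanced Input mapping context on its player controller.
; IA_Move adds movement input along X and snaps control rotation yaw to face forward or backward based on the input sign.
; IA_Jump starts the jump on Started and stops it on Canceled.
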(event Input|EnhancedActionEvents|EnhancedInputActionIA_Move
  (params (ActionValue :type Float%20%28double-precision%29) (ElapsedSeconds :type Float%20%28double-precision%29) (TriggeredSeconds :type Float%20%28double-precision%29) (InputAction :type Input%20Action%20Object%20Reference :default "/Game/Blueprints/Character/Input/Action/IA_Move.IA_Move"))
  ;[1 0.9387 0.01181 0.5] Player Input
  (Pawn|Input|AddMovementInput "1.000000,0.000000,0.000000" ActionValue false)
  (Pawn|SetControlRotation (Pawn|GetController) (select (< ActionValue 0.0) (Math|Rotator|MakeRotator 0.0 0.0 -1.8e+02) (Math|Rotator|MakeRotator 0.0 0.0 0.0))))

(event Input|EnhancedActionEvents|EnhancedInputActionIA_Jump
  (params (ActionValue :type Boolean) (ElapsedSeconds :type Float%20%28double-precision%29) (TriggeredSeconds :type Float%20%28double-precision%29) (InputAction :type Input%20Action%20Object%20Reference :default "/Game/Blueprints/Character/Input/Action/IA_Jump.IA_Jump"))
  ;[1 0.9387 0.01181 0.5] Player Input
  (:Started
    (Character|Jump))
  (:Canceled
    (Character|StopJumping)))

(event EventBeginPlay
  (|CallParentFunction)
  ;[0.874 0.8012 0 0.5] Setting up Input Mapping Context
  (bind _asplayer_controller (Utilities|Casting|CastToPlayerController (Pawn|GetController)))
  (Input|AddMappingContext (PlayerController|LocalPlayerSubsystems|GetEnhancedInputLocalPlayerSubsystem _asplayer_controller) "/Game/Blueprints/Character/Input/IMC_Player.IMC_Player" 0 "(bIgnoreAllPressedKeysUntilRelease=True,bForceImmediately=False,bNotifyUserSettings=False)"))

(event Collision|EventActorBeginOverlap
  (params (OtherActor :type Actor%20Object%20Reference))
  (|CallParentFunction OtherActor) ; This node is disabled and will not be called.\nDrag off pins to build functionality.
)

(event EventTick
  (params (DeltaSeconds :type Float%20%28single-precision%29))
  (|CallParentFunction DeltaSeconds) ; This node is disabled and will not be called.\nDrag off pins to build functionality.
)

(fn ConstructionScript
  (|CallParentFunction))